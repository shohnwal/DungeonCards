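; Game mode for a multiplayer card game, handling each player's deck, hand and played card on the server.
; Deck creation adds ten cards built from data table row 0 to the PlayerState, and drawing moves the first into the hand.
; Play requests check hand membership, set the played card and notify the client through PlayerController events.
; TryUseCard switches on card type but has no actions yet.
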(event Custom|TryUseCard
  (params (CardToUse :type DC%20Card%20Object%20Reference) (DCPlayerController :type DC%20Player%20Controller%20BP%20Object%20Reference))
  ;[1 1 1] Check if player has the card
  (bind _asdcplayer_state_bp (Utilities|Casting|CastToDCPlayerState_BP (Variables|/Script/Engine.Controller|GetPlayerState DCPlayerController)))
  (if (Utilities|Array|ContainsItem (Variables|/Game/Blueprint/GameBase/Game/DCPlayerState_BP.DCPlayerState_BP_C|GetHand _asdcplayer_state_bp) CardToUse)
    (switch Utilities|FlowControl|Switch|SwitchonECardType (Variables|/Script/DungeonCards.DCCard|GetCardType CardToUse))))

(event Custom|TryPlayCard
  (params (CardToPlay :type DC%20Card%20Object%20Reference) (DCPlayerController :type DC%20Player%20Controller%20BP%20Object%20Reference))
  (bind _success (CallFunction|CheckifCanPlayCard CardToPlay DCPlayerController))
  (if _success
    (CallFunction|PlayCard CardToPlay DCPlayerController)
    (else
      (Default|CLIENTNotifyCantPlayThisCard DCPlayerController))))

(event Custom|SERVER_DrawCard
  (params (DCPlayerController :type DC%20Player%20Controller%20BP%20Object%20Reference))
  (bind _asdcplayer_state_bp (Utilities|Casting|CastToDCPlayerState_BP (Variables|/Script/Engine.Controller|GetPlayerState DCPlayerController)))
  (if (> (Utilities|Array|Length (Variables|/Game/Blueprint/GameBase/Game/DCPlayerState_BP.DCPlayerState_BP_C|GetDeck _asdcplayer_state_bp)) 0)
    (Utilities|Array|Add (Variables|/Game/Blueprint/GameBase/Game/DCPlayerState_BP.DCPlayerState_BP_C|GetHand _asdcplayer_state_bp) (Utilities|Array|Get(acopy) (Variables|/Game/Blueprint/GameBase/Game/DCPlayerState_BP.DCPlayerState_BP_C|GetDeck _asdcplayer_state_bp)))
    (Utilities|Array|RemoveIndex (Variables|/Game/Blueprint/GameBase/Game/DCPlayerState_BP.DCPlayerState_BP_C|GetDeck _asdcplayer_state_bp))
    (Default|CLIENTUpdateHandCards DCPlayerController)))

(event Custom|SERVER_CreateCards
  (params (DCPlayerController :type DC%20Player%20Controller%20BP%20Object%20Reference))
  (bind _asdcplayer_state_bp (Utilities|Casting|CastToDCPlayerState_BP (Variables|/Script/Engine.Controller|GetPlayerState DCPlayerController)))
  (for _index (range 0 9)
    (bind _newcard (CallFunction|CreatePlayCard))
    (Utilities|IsValid _newcard
      (:Is%20Valid
        (Utilities|Array|Add (Variables|/Game/Blueprint/GameBase/Game/DCPlayerState_BP.DCPlayerState_BP_C|GetDeck _asdcplayer_state_bp) _newcard))
      (:Is%20Not%20Valid
        (Development|PrintString "GameMode : CreatedCard not valid")))))

(event EventBeginPlay)

(event EventTick
  (params (DeltaSeconds :type Float%20%28single-precision%29)))

(event EventPostLogin
  (params (NewPlayer :type Player%20Controller%20Object%20Reference))
  (bind _returnvalue (Class|GameplayStatics|GetPlayerControllerID NewPlayer))
  (if (== _returnvalue 0)
    (Development|PrintString "IsServer")
    (else
      (Development|PrintString "IsClient"))))

(fn ConstructionScript)

(fn CheckifCanPlayCard
  (params (CardToPlay :type DC%20Card%20Object%20Reference) (DCPlayerController :type DC%20Player%20Controller%20BP%20Object%20Reference))
  (bind _asdcplayer_state_bp (Utilities|Casting|CastToDCPlayerState_BP (Variables|/Script/Engine.Controller|GetPlayerState DCPlayerController))
    (:then
      (return (Utilities|Array|ContainsItem (Variables|/Game/Blueprint/GameBase/Game/DCPlayerState_BP.DCPlayerState_BP_C|GetHand _asdcplayer_state_bp) CardToPlay)))
    (:CastFailed
      (return false))))

(fn PlayCard
  (params (CardToPlay :type DC%20Card%20Object%20Reference) (DCPlayerController :type DC%20Player%20Controller%20BP%20Object%20Reference))
  (bind _asdcplayer_state_bp (Utilities|Casting|CastToDCPlayerState_BP (Variables|/Script/Engine.Controller|GetPlayerState DCPlayerController)))
  (Utilities|Array|RemoveItem (Variables|/Game/Blueprint/GameBase/Game/DCPlayerState_BP.DCPlayerState_BP_C|GetHand _asdcplayer_state_bp) CardToPlay)
  (bind _output_get (Variables|/Game/Blueprint/GameBase/Game/DCPlayerState_BP.DCPlayerState_BP_C|SetCurrentlyPlayedCard _asdcplayer_state_bp CardToPlay))
  (Default|CLIENTMoveCardfromHandtoPlayedCardSlot DCPlayerController _output_get))

(fn CreatePlayCard
  (params (CardId :type Integer))
  (bind _returnvalue (Utilities|GetDataTableRow "/Game/Blueprint/GameBase/Game/CardsDataTable.CardsDataTable" (Utilities|String|StringToName (Utilities|String|ToString(Integer) CardId)))
    (:then
      (bind _returnvalue_2 (Class|DCGameMode|CreateCard self (.CardClass (Utilities|Struct|BreakCardsDataTblEntry _returnvalue))))
      (return _returnvalue_2))))