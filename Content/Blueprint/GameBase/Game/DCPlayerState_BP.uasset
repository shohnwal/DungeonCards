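; Player state for a turn-based card game, holding a player's hand and graveyard.
; Helper functions add and remove hand cards and move them to the graveyard.
; UpdateTurnStatus compares PlayerType to the new current player, then begins or ends the turn on player controller 0.
; SERVER_ConfirmAssetsLoaded tells DCGameMode_BP to begin the game.
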(event Custom|SERVER_ConfirmAssetsLoaded
  (bind _asdcgame_mode_bp (Utilities|Casting|CastToDCGameMode_BP (Game|GetGameMode)))
  (Default|BeginGame _asdcgame_mode_bp))

(event EventBeginPlay)

(event EventTick
  (params (DeltaSeconds :type Float%20%28single-precision%29)))

(fn ConstructionScript)

(fn UpdateTurnStatus
  (params (NewCurrentPlayer :type EPlayerType%20Enum :default "HERO"))
  (bind _asdcplayer_controller_bp (Utilities|Casting|CastToDCPlayerController_BP (Game|GetPlayerController 0)))
  (if (Utilities|Enum|Equal(Enum) (Variables|Default|GetPlayerType) NewCurrentPlayer)
    (Default|BeginTurn _asdcplayer_controller_bp)
    (else
      (Default|EndTurn _asdcplayer_controller_bp))))

(fn RemoveCardfromHand
  (params (CardToRemove :type DC%20Card%20Object%20Reference))
  (Utilities|Array|RemoveItem (Variables|Default|GetHand) CardToRemove)
  (return))

(fn AddCardtoHand
  (params (CardToAdd :type DC%20Card%20Object%20Reference))
  (Utilities|Array|Add (Variables|Default|GetHand) CardToAdd)
  (return))

(fn AddCardtoGraveYard
  (params (CardToAdd :type DC%20Card%20Object%20Reference))
  (Utilities|Array|Add (Variables|Default|GetGraveyard) CardToAdd)
  (return))

(fn MoveCardfromHandtoGraveyard
  (params (Card :type DC%20Card%20Object%20Reference))
  (CallFunction|RemoveCardfromHand Card)
  (CallFunction|AddCardtoGraveYard Card)
  (return))