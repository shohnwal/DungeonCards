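; Player controller for a turn-based multiplayer card game, handling camera, HUD and card-play requests.
; On the local client it spawns a camera pawn with pan, right-drag rotate and wheel zoom, plus the test HUD.
; Server events forward card plays and turn endings to DCGameMode_BP, client events update the HUD, and ControlMode tracks turn state.
; Hover tracing and debug keys are included; card cancelling is stubbed.
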(event Custom|TryEndTurn
  ;[0 0 0] Turn mechanics
  (switch Utilities|FlowControl|Switch|SwitchonEControlMode (Variables|Default|GetControlMode)
    (:DEFAULTCONTROLS
      (Variables|Default|SetControlMode "WAITINGFORRESPONSE")
      (CallFunction|SERVERRequestEndTurn))))

(event Custom|SERVER_TryToPlayCard
  (params (CardToPlay :type DC%20Card%20Object%20Reference))
  ;[0 0 0] Card Playing
  ;;[1 1 1] Server
  (bind _asdcgame_mode_bp (Utilities|Casting|CastToDCGameMode_BP (Game|GetGameMode self)))
  (Default|TryPlayCard _asdcgame_mode_bp CardToPlay self))

(event Custom|CLIENT_UpdateHandCards
  ;[0 0 0] Card Playing
  ;;[1 1 1] Client
  (bind _asw_test_hud_bp (Utilities|Casting|CastToW_TestHud_BP (Variables|Default|GetMainUMGWidget)))
  (Default|UpdateHandCards _asw_test_hud_bp))

(event Custom|CLIENT_NotifyCantPlayThisCard
  ;[0 0 0] Card Playing
  ;;[1 1 1] Client
  (Development|PrintString "Can't play this card"))

(event Custom|CancelCurrentCardUse)

(event Custom|SERVER_CancelCurrentCardUse)

(event Custom|CLIENT_ConfirmCancelCurrentCardUse)

(event Custom|SERVER_RequestEndTurn
  ;[0 0 0] Turn mechanics
  (bind _asdcgame_mode_bp (Utilities|Casting|CastToDCGameMode_BP (Game|GetGameMode)))
  (Default|TrytoEndTurn _asdcgame_mode_bp (Variables|Default|GetPlayerType)))

(event Custom|CLIENT_MoveCardFromHandToPlayedCardSlot
  (params (CardToRemove :type DC%20Card%20Object%20Reference))
  ;[0 0 0] Card Playing
  ;;[1 1 1] Client
  (bind _asw_test_hud_bp (Utilities|Casting|CastToW_TestHud_BP (Variables|Default|GetMainUMGWidget)))
  (Default|MoveCardfromHandtoPlayedCardSlot _asw_test_hud_bp CardToRemove))

(event Custom|C_TryPlayCard
  (params (CardToPlay :type DC%20Card%20Object%20Reference))
  ;[0 0 0] Card Playing
  ;;[1 1 1] Client
  (CallFunction|SERVERTrytoPlayCard CardToPlay))

(event EventBeginPlay
  ;[0 0 0] Client
  ;;[1 1 1] BeginPlay
  (if (Pawn|IsLocalPlayerController self)
    (Development|PrintString "local")
    (CallFunction|CreateCamera)
    (CallFunction|SetupHud)
    (else
      (Development|PrintString "not local"))))

(event EventTick
  (params (DeltaSeconds :type Float%20%28single-precision%29))
  (bind _array (Utilities|Array|MakeArray "ObjectTypeQuery3"))
  (bind (_hitresult _returnvalue) (Class|PlayerController|GetHitResultUnderCursorforObjects _array true))
  ;[1 1 1] Tick
  (if _returnvalue
    (Variables|Default|SetHoveredOverActor (.hitactor _hitresult))
    (else
      (Variables|Default|SetHoveredOverActor 0))))

(event Input|AxisEvents|InputAxisMoveForward
  (params (AxisValue :type Float%20%28single-precision%29))
  (bind _mycameraactor (Variables|Default|GetMyCameraActor))
  ;[0 0 0] Client
  ;;[1 1 1] Camera controls
  (Utilities|IsValid _mycameraactor
    (:Is%20Valid
      (Transformation|AddRelativeLocation (Variables|/Script/Engine.Actor|GetRootComponent _mycameraactor) (* (Math|Vector|GetForwardVector (Math|Rotator|MakeRotator 0.0 0.0 (.yaw (Camera|GetCameraRotation (Game|GetPlayerCameraManager 0))))) (* AxisValue 1e+01)) false false))))

(event Input|AxisEvents|InputAxisMoveRight
  (params (AxisValue :type Float%20%28single-precision%29))
  (bind _mycameraactor (Variables|Default|GetMyCameraActor))
  ;[0 0 0] Client
  ;;[1 1 1] Camera controls
  (Utilities|IsValid _mycameraactor
    (:Is%20Valid
      (Transformation|AddRelativeLocation (Variables|/Script/Engine.Actor|GetRootComponent _mycameraactor) (* (Math|Vector|GetRightVector (Math|Rotator|MakeRotator 0.0 0.0 (.yaw (Camera|GetCameraRotation (Game|GetPlayerCameraManager 0))))) (* AxisValue 1e+01)) false false))))

(event Input|MouseEvents|MouseX
  (params (AxisValue :type Float%20%28single-precision%29))
  (bind (_sizex _sizey) (HUD|GetViewportSize))
  (bind _mycameraactor (Variables|Default|GetMyCameraActor))
  (bind _springarm (Variables|/Game/Blueprint/DCCameraPawn.DCCameraPawn_C|GetSpringArm _mycameraactor))
  (bind _relativerotation (Variables|/Script/Engine.SceneComponent|GetRelativeRotation _springarm))
  ;[0 0 0] Client
  ;;[1 1 1] Camera controls
  (if (Variables|Default|GetRightMouseButtonClicked)
    (Class|PlayerController|SetMouseLocation (/ _sizex 2) (/ _sizey 2))
    (Transformation|SetRelativeRotation _springarm (Math|Rotator|MakeRotator 0.0 (Math|Float|Clamp(Float) (+ (.pitch _relativerotation) (* (stale Input|MouseEvents|MouseY AxisValue) 1.0)) -8e+01 -2e+01) (+ (.yaw _relativerotation) (* AxisValue 2.0))) false false)))

(event Input|MouseEvents|MouseWheelAxis
  (params (AxisValue :type Float%20%28single-precision%29))
  (bind _mycameraactor (Variables|Default|GetMyCameraActor))
  (bind _springarm (Variables|/Game/Blueprint/DCCameraPawn.DCCameraPawn_C|GetSpringArm _mycameraactor))
  ;[0 0 0] Client
  ;;[1 1 1] Camera controls
  (Variables|/Script/Engine.SpringArmComponent|SetTargetArmLength _springarm (Math|Float|Clamp(Float) (+ (* AxisValue -1e+02) (Variables|/Script/Engine.SpringArmComponent|GetTargetArmLength _springarm)) 2e+02 3e+03)))

(event Input|MouseEvents|MouseY
  (params (AxisValue :type Float%20%28single-precision%29))
  (bind (_sizex _sizey) (HUD|GetViewportSize))
  (bind _mycameraactor (Variables|Default|GetMyCameraActor))
  (bind _springarm (Variables|/Game/Blueprint/DCCameraPawn.DCCameraPawn_C|GetSpringArm _mycameraactor))
  (bind _relativerotation (Variables|/Script/Engine.SceneComponent|GetRelativeRotation _springarm))
  ;[0 0 0] Client
  ;;[1 1 1] Camera controls
  (if (Variables|Default|GetRightMouseButtonClicked)
    (Class|PlayerController|SetMouseLocation (/ _sizex 2) (/ _sizey 2))
    (Transformation|SetRelativeRotation _springarm (Math|Rotator|MakeRotator 0.0 (Math|Float|Clamp(Float) (+ (.pitch _relativerotation) (* AxisValue 1.0)) -8e+01 -2e+01) (+ (.yaw _relativerotation) (* (stale Input|MouseEvents|MouseX AxisValue) 2.0))) false false)))

(event Input|KeyboardEvents|Q
  (params (Key :type Key%20Structure))
  ;[0 0 0] Client
  ;;[1 1 1] Quit game
  (:Pressed
    (Game|QuitGame self "Quit")))

(event Input|KeyboardEvents|P
  (params (Key :type Key%20Structure))
  ;[0 0 0] Client
  (:Pressed
    (bind _returnvalue (Class|NavigationSystem|FindPathtoLocationSynchronously (Math|Vector|MakeVector 0.0 0.0 0.0) (.location (.HitResult (Game|Player|GetHitResultUnderCursorbyChannel "TraceTypeQuery1" true))) self))
    (for _array_element (Variables|/Script/Engine.NavigationPath|GetPathPoints _returnvalue)
      (Rendering|Debug|DrawDebugSphere _array_element 1e+01 12 "(R=1.000000,G=1.000000,B=1.000000,A=1.000000)" 2.0 1.0))))

(event Input|MouseEvents|LeftMouseButton
  (params (Key :type Key%20Structure))
  (bind _hoveredoveractor (Variables|Default|GetHoveredOverActor))
  ;[0 0 0] Client
  ;;[1 1 1] Left Mouse Button
  (:Pressed
    (Utilities|IsValid _hoveredoveractor
      (:Is%20Valid
        (Development|PrintString (Class|KismetSystemLibrary|GetPathName _hoveredoveractor))))))

(event Input|MouseEvents|RightMouseButton
  (params (Key :type Key%20Structure))
  (bind (_locationx _locationy) (Game|Player|GetMousePosition))
  ;[0 0 0] Client
  ;;[1 1 1] Camera controls
  (:Pressed
    (Variables|Default|SetSavedMousePos (Math|Vector2D|MakeVector2D _locationx _locationy))
    (Variables|Default|SetRightMouseButtonClicked true)
    (Variables|Default|SetbShowMouseCursor false))
  (:Released
    (Class|PlayerController|SetMouseLocation (Math|Float|Truncate (.x (Variables|Default|GetSavedMousePos))) (Math|Float|Truncate (.y (Variables|Default|GetSavedMousePos))))
    (Variables|Default|SetRightMouseButtonClicked false)
    (Variables|Default|SetbShowMouseCursor true)))

(event Input|KeyboardEvents|Left
  (params (Key :type Key%20Structure))
  ;[0 0 0] Client
  (:Pressed
    (Development|PrintString "is local player controller?")
    (Development|PrintString (Utilities|String|ToString(Boolean) (Pawn|IsLocalPlayerController)))
    (Development|PrintString "Has authority?")
    (Development|PrintString (Utilities|String|ToString(Boolean) (Ability|HasAuthority)))))

(fn ConstructionScript)

(fn CreateCamera
  (bind _returnvalue (Game|SpawnActorfromClass "/Game/Blueprint/DCCameraPawn.DCCameraPawn_C" (Math|Transform|MakeTransform "0, 0,50.000000") "AlwaysSpawn" self 0))
  (Game|Player|SetViewTargetwithBlend _returnvalue 0.0 "VTBlend_Linear" 0.0 false)
  (Variables|Default|SetMyCameraActor _returnvalue)
  (return))

(fn SetupHud
  (bind _returnvalue (UserInterface|CreateWidget "/Game/Blueprint/Ui/Game/W_TestHud_BP.W_TestHud_BP_C" self))
  (UserInterface|Viewport|AddtoViewport _returnvalue 0)
  (Variables|Default|SetMainUMGWidget _returnvalue))

(fn BeginTurn
  (Variables|Default|SetControlMode "DEFAULTCONTROLS")
  (Development|PrintString "it's my turn! :)" true true "(R=0.000000,G=0.660000,B=1.000000,A=1.000000)" 2e+01))

(fn EndTurn
  (Variables|Default|SetControlMode "NOGAMEPLAY")
  (Development|PrintString "not my turn..." true true "(R=0.000000,G=0.660000,B=1.000000,A=1.000000)" 2e+01))