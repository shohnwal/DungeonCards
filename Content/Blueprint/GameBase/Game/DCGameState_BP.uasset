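; DCGameState_BP is the game state of a turn-based card game, relaying turn and phase changes to each client.
; Multicast events pass the active player to the local DCPlayerState_BP, or store the new phase and call CBeginPhase on the local DCPlayerController_BP, both reached through player index 0.
; It also keeps a stack of currently played cards and prints debug messages; ResumePhase and EndTurn multicasts are empty stubs.
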(event Custom|MULTICAST_SwitchTurn
  (params (NewCurrentPlayer :type EPlayerType%20Enum :default "HERO"))
  (bind _asdcplayer_state_bp (Utilities|Casting|CastToDCPlayerState_BP (Variables|/Script/Engine.Controller|GetPlayerState (Game|GetPlayerController 0))))
  (Default|UpdateTurnStatus _asdcplayer_state_bp NewCurrentPlayer))

(event Custom|MULTICAST_BeginGame
  (params (ActivePlayer :type EPlayerType%20Enum :default "HERO"))
  (bind _asdcplayer_state_bp (Utilities|Casting|CastToDCPlayerState_BP (Variables|/Script/Engine.Controller|GetPlayerState (Game|GetPlayerController 0))))
  (Default|UpdateTurnStatus _asdcplayer_state_bp ActivePlayer))

(event Custom|MULTICAST_AnnounceNewPhase
  (params (NewTurnPhase :type ETurnPhase%20Enum :default "NewEnumerator1"))
  (Variables|Default|SetCurrentPhase NewTurnPhase)
  (Development|PrintString (Utilities|String|Append "Client : New phase : " (Utilities|String|EnumtoString NewTurnPhase)) true true "(R=0.510417,G=0.032757,B=0.000000,A=1.000000)" 3e+01)
  (bind _asdcplayer_controller_bp (Utilities|Casting|CastToDCPlayerController_BP (Game|GetPlayerController 0)))
  (Default|CBeginPhase _asdcplayer_controller_bp NewTurnPhase))

(event Custom|MULTICAST_ResumePhase
  (params (ResumeTurnPhase :type ETurnPhase%20Enum :default "NewEnumerator1")))

(event Custom|MULTICAST_EndTurn)

(event EventBeginPlay
  (bind _asdcplayer_controller_bp (Utilities|Casting|CastToDCPlayerController_BP (Game|GetPlayerController 0)))
  (Variables|Default|SetMyPlayerController _asdcplayer_controller_bp)
  (Development|PrintString "gamestate set new player controller"))

(event EventTick
  (params (DeltaSeconds :type Float%20%28single-precision%29)))

(fn ConstructionScript)

(fn AddCardtoPlayedCardStack
  (params (PlayedCard :type DC%20Card%20Object%20Reference))
  (bind _returnvalue (Utilities|Array|Add (Variables|Default|GetCurrentlyPlayedCards) PlayedCard))
  (Development|PrintString (Utilities|String|Append "Now this many cards on played card stack : " (Utilities|String|ToString(Integer) _returnvalue)))
  (return))