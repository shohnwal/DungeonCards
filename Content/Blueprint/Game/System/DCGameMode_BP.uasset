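; Server game mode for a two-player turn-based card game pitting a Hero against a Dungeon Master.
; PostLogin assigns roles, then with two players builds placeholder decks, deals hands and starts turns.
; Once both clients confirm, phases chain from upkeep through perma effects and draw to action, multicast via the game state; upkeep and perma effects are stubs.
; It validates card plays, relays them to both clients and swaps priority at turn end.
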(event Custom|SERVER_DrawCard
  (params (DCPlayerController :type DC%20Player%20Controller%20BP%20Object%20Reference))
  (bind _asdcplayer_state_bp (Utilities|Casting|CastToDCPlayerState_BP (Variables|/Script/Engine.Controller|GetPlayerState DCPlayerController)))
  (if (> (Utilities|Array|Length (Variables|/Game/Blueprint/Game/System/DCPlayerState_BP.DCPlayerState_BP_C|GetDeck _asdcplayer_state_bp)) 0)
    (Utilities|Array|Add (Variables|/Game/Blueprint/Game/System/DCPlayerState_BP.DCPlayerState_BP_C|GetHand _asdcplayer_state_bp) (Utilities|Array|Get(acopy) (Variables|/Game/Blueprint/Game/System/DCPlayerState_BP.DCPlayerState_BP_C|GetDeck _asdcplayer_state_bp)))
    (Utilities|Array|RemoveIndex (Variables|/Game/Blueprint/Game/System/DCPlayerState_BP.DCPlayerState_BP_C|GetDeck _asdcplayer_state_bp))))

(event Custom|BeginNewPhase
  (params (NewPhase :type ETurnPhase%20Enum :default "NewEnumerator1"))
  (Development|PrintString (Utilities|String|Append "SERVER : Begin new phase : " (Utilities|String|EnumtoString NewPhase)) true true "(R=0.000000,G=0.307292,B=0.017300,A=1.000000)" 3e+01)
  (bind _asdcgame_state_bp (Utilities|Casting|CastToDCGameState_BP (Game|GetGameState)))
  ;[1 1 1] Notify clients that new phase has begun
  (Default|MULTICASTBeginNewPhase _asdcgame_state_bp NewPhase)
  (Utilities|FlowControl|Delay 0.1)
  (switch Utilities|FlowControl|Switch|SwitchonETurnPhase NewPhase
    (:NewEnumerator1
      ;[1 1 1] Do new phase stuff
      (CallFunction|PhaseUpkeepBegin))
    (:NewEnumerator2
      (CallFunction|PhasePermaEffectsBegin))
    (:NewEnumerator3
      (CallFunction|PhaseDrawCardBegin))
    (:NewEnumerator4
      (CallFunction|PhaseActionBegin))))

(event EventBeginPlay)

(event EventTick
  (params (DeltaSeconds :type Float%20%28single-precision%29)))

(event EventPostLogin
  (params (NewPlayer :type Player%20Controller%20Object%20Reference))
  (bind _returnvalue (Class|GameModeBase|GetNumPlayers))
  (Development|PrintString (Utilities|String|ToString(Integer) _returnvalue) true true "(R=0.000000,G=0.660000,B=1.000000,A=1.000000)" 6e+01)
  (bind _asdcplayer_controller_bp (Utilities|Casting|CastToDCPlayerController_BP NewPlayer))
  (bind _returnvalue_2 (Class|GameplayStatics|GetPlayerControllerID NewPlayer))
  (switch int _returnvalue_2
    (:Default
      (CallFunction|SetupPlayer _asdcplayer_controller_bp "DUNGEONMASTER" false)
      (bind _returnvalue_3 (Class|GameModeBase|GetNumPlayers))
      (if (== _returnvalue_3 2)
        (Development|PrintString "Enough players connected, game should start" :!label _label)
        (CallFunction|PrepareGame)
        (Utilities|FlowControl|Delay 0.2)
        (CallFunction|BeginGame)))
    (:0
      (CallFunction|SetupPlayer _asdcplayer_controller_bp "HERO" true)
      (bind _returnvalue_4 (Class|GameModeBase|GetNumPlayers))
      (if (== _returnvalue_4 2)
        (goto _label)))))

(event EventOnLogout
  (params (ExitingController :type Controller%20Object%20Reference))
  (bind _returnvalue (Class|GameModeBase|GetNumPlayers)))

(fn ConstructionScript)

(fn CheckifCanPlayCard
  (params (CardToPlay :type DC%20Card%20Base%20BP%20Object%20Reference) (DCPlayerController :type DC%20Player%20Controller%20BP%20Object%20Reference))
  (bind _asdcplayer_state_bp (Utilities|Casting|CastToDCPlayerState_BP (Variables|/Script/Engine.Controller|GetPlayerState DCPlayerController))
    (:then
      (return (Utilities|Array|ContainsItem (Variables|/Game/Blueprint/Game/System/DCPlayerState_BP.DCPlayerState_BP_C|GetHand _asdcplayer_state_bp) CardToPlay)))
    (:CastFailed
      (return false))))

(fn PlayCard
  (params (CardToPlay :type DC%20Card%20Base%20BP%20Object%20Reference) (DCPlayerController :type DC%20Player%20Controller%20BP%20Object%20Reference))
  (bind _activeplayercontroller (Variables|Default|GetActivePlayerController))
  (bind _success (CallFunction|CheckifCanPlayCard CardToPlay DCPlayerController))
  (if _success
    (bind _asdcplayer_state_bp (Utilities|Casting|CastToDCPlayerState_BP (Variables|/Script/Engine.Controller|GetPlayerState DCPlayerController)))
    (Default|RemoveCardfromHand _asdcplayer_state_bp CardToPlay)
    (Default|CLIENTRemoveCardfromHand DCPlayerController CardToPlay)
    (bind _asdcgame_state_bp (Utilities|Casting|CastToDCGameState_BP (Game|GetGameState)))
    (Default|AddCardtoPlayedCardStack _asdcgame_state_bp CardToPlay)
    (Default|CLIENTDisplayNewPlayedCard (Variables|Default|GetPassivePlayerController) CardToPlay)
    (Default|CLIENTDisplayNewPlayedCard _activeplayercontroller CardToPlay)
    (switch Utilities|FlowControl|Switch|SwitchonECardType (Variables|/Script/DungeonCards.DCCard|GetCardType CardToPlay)
      (:SUMMONMINION
        (Default|CLIENTAskforSummonLocation _activeplayercontroller)))
    (else
      (Default|CLIENTNotifyCantPlayThisCard DCPlayerController))))

(fn CreatePlayCard
  (params (CardId :type Integer))
  (bind _returnvalue (Utilities|GetDataTableRow "/Game/Blueprint/Game/System/CardsDataTable.CardsDataTable" (Utilities|String|StringToName (Utilities|String|ToString(Integer) CardId)))
    (:then
      (bind _returnvalue_2 (Class|DCGameMode|CreateCard self (Utilities|Struct|BreakCardsDataTblEntry _returnvalue)))
      (return _returnvalue_2))))

(fn TrytoEndTurn
  (Variables|Default|SetPassivePlayerReadyForTurnStart false)
  (Variables|Default|SetActivePlayerReadyForTurnStart false)
  (Default|CLIENTFinalizeEndTurn (Variables|Default|GetPassivePlayerController))
  (Default|CLIENTFinalizeEndTurn (Variables|Default|GetActivePlayerController))
  (bind (_newactiveplayer _newpassiveplayer) (CallFunction|SwapPlayerPriority))
  (Default|CLIENTBeginPassiveTurn _newpassiveplayer)
  (Default|CLIENTBeginActiveTurn _newactiveplayer))

(fn SwapPlayerPriority
  (LocalVariables|SetPlayerController_Temp (Variables|Default|GetActivePlayerController))
  (bind _output_get (Variables|Default|SetActivePlayerController (Variables|Default|GetPassivePlayerController)))
  (Variables|/Game/Blueprint/Game/System/DCPlayerController_BP.DCPlayerController_BP_C|SetItsMyTurn _output_get true)
  (bind _output_get_2 (Variables|Default|SetPassivePlayerController (LocalVariables|GetPlayerController_Temp)))
  (Variables|/Game/Blueprint/Game/System/DCPlayerController_BP.DCPlayerController_BP_C|SetItsMyTurn _output_get_2 false)
  (Variables|Default|SetActivePlayerReadyForTurnStart false)
  (Variables|Default|SetPassivePlayerReadyForTurnStart false)
  (return _output_get _output_get_2))

(fn SetupPlayer
  (params (DCPlayerController :type DC%20Player%20Controller%20BP%20Object%20Reference) (PlayerType :type EPlayerType%20Enum :default "HERO") (Active :type Boolean))
  (bind _asdcplayer_state_bp (Utilities|Casting|CastToDCPlayerState_BP (Variables|/Script/Engine.Controller|GetPlayerState DCPlayerController)))
  (Variables|/Game/Blueprint/Game/System/DCPlayerState_BP.DCPlayerState_BP_C|SetPlayerType _asdcplayer_state_bp PlayerType)
  (if Active
    (Variables|Default|SetActivePlayerController DCPlayerController)
    (else
      (Variables|Default|SetPassivePlayerController DCPlayerController))))

(fn PhaseUpkeepBegin
  (Utilities|Casting|CastToDCGameState_BP (Game|GetGameState))
  ;[1 1 1] Make list of all upkeep objects of player
  (Utilities|Array|Clear (Variables|Default|GetUpkeepCardsArray))
  ;[1 1 1] Check if upkeep list size has elements
  (if (not false)
    ;[1 1 1] No upkeep cards found, go on to perma effects phase
    (CallFunction|BeginNewPhase "NewEnumerator2")))

(fn PhaseUpkeepContinue)

(fn PhasePermaEffectsBegin
  (CallFunction|BeginNewPhase "NewEnumerator3"))

(fn PhasePermaEffectsContinue)

(fn PhaseDrawCardBegin
  (bind _asdcplayer_state_bp (Utilities|Casting|CastToDCPlayerState_BP (Variables|/Script/Engine.Controller|GetPlayerState (Variables|Default|GetActivePlayerController))))
  (if (> (Utilities|Array|Length (Variables|/Game/Blueprint/Game/System/DCPlayerState_BP.DCPlayerState_BP_C|GetDeck _asdcplayer_state_bp)) 0)
    (Utilities|Array|Add (Variables|/Game/Blueprint/Game/System/DCPlayerState_BP.DCPlayerState_BP_C|GetHand _asdcplayer_state_bp) (Utilities|Array|Get(acopy) (Variables|/Game/Blueprint/Game/System/DCPlayerState_BP.DCPlayerState_BP_C|GetDeck _asdcplayer_state_bp)))
    (Utilities|Array|RemoveIndex (Variables|/Game/Blueprint/Game/System/DCPlayerState_BP.DCPlayerState_BP_C|GetDeck _asdcplayer_state_bp))
    (CallFunction|BeginNewPhase "NewEnumerator4")
    (else
      (Development|PrintString "no cards"))))

(fn PhaseDrawCardContinue)

(fn PhaseActionBegin)

(fn PhaseActionContinue)

(fn BeginGame
  (Default|CLIENTBeginPassiveTurn (Variables|Default|GetPassivePlayerController))
  (Default|CLIENTBeginActiveTurn (Variables|Default|GetActivePlayerController))
  (return))

(fn CreateCardDeckforPlayer
  (params (DCPlayerController :type DC%20Player%20Controller%20BP%20Object%20Reference))
  (bind _asdcplayer_state_bp (Utilities|Casting|CastToDCPlayerState_BP (Variables|/Script/Engine.Controller|GetPlayerState DCPlayerController))
    (:then
      (for _index (range 0 50)
        (bind _newcard (CallFunction|CreatePlayCard 1))
        (bind _asdccard_base_bp (Utilities|Casting|CastToDCCard_Base_BP _newcard))
        (Utilities|Array|Add (Variables|/Game/Blueprint/Game/System/DCPlayerState_BP.DCPlayerState_BP_C|GetDeck _asdcplayer_state_bp) _asdccard_base_bp)))
    (:CastFailed
      _))
  (return))

(fn DrawCard
  (params (DCPlayerController :type DC%20Player%20Controller%20BP%20Object%20Reference))
  (bind _asdcplayer_state_bp (Utilities|Casting|CastToDCPlayerState_BP (Variables|/Script/Engine.Controller|GetPlayerState DCPlayerController)))
  (if (> (Utilities|Array|Length (Variables|/Game/Blueprint/Game/System/DCPlayerState_BP.DCPlayerState_BP_C|GetDeck _asdcplayer_state_bp)) 0)
    (Utilities|Array|Add (Variables|/Game/Blueprint/Game/System/DCPlayerState_BP.DCPlayerState_BP_C|GetHand _asdcplayer_state_bp) (Utilities|Array|Get(acopy) (Variables|/Game/Blueprint/Game/System/DCPlayerState_BP.DCPlayerState_BP_C|GetDeck _asdcplayer_state_bp)))
    (Utilities|Array|RemoveIndex (Variables|/Game/Blueprint/Game/System/DCPlayerState_BP.DCPlayerState_BP_C|GetDeck _asdcplayer_state_bp))))

(fn PrepareGame
  (CallFunction|CreateCardDeckforPlayer (Variables|Default|GetPassivePlayerController))
  (CallFunction|CreateCardDeckforPlayer (Variables|Default|GetActivePlayerController))
  (for _index (range 0 9)
    (CallFunction|DrawCard (Variables|Default|GetActivePlayerController))
    (CallFunction|DrawCard (Variables|Default|GetPassivePlayerController))))

(fn PlayerConfirmTurnStart
  (params (ActivePlayer :type Boolean))
  (if ActivePlayer
    (Variables|Default|SetActivePlayerReadyForTurnStart true)
    (else
      (Variables|Default|SetPassivePlayerReadyForTurnStart true)))
  (if (and (Variables|Default|GetPassivePlayerReadyForTurnStart) (Variables|Default|GetActivePlayerReadyForTurnStart))
    (CallFunction|BeginNewPhase "NewEnumerator1")))