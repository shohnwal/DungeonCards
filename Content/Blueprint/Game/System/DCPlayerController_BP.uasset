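; Player controller for a turn-based card game on tiled terrain, handling camera, HUD, input and client-server turn flow.
; It spawns an orbit, pan and zoom camera, and highlights the hovered tile through custom depth.
; SERVER events forward turns and card plays to DCGameMode_BP; CLIENT events update the HUD and control mode.
; Control mode gates turn ending and click-to-summon, which spawns a fixed test creature; debug keys exercise pathfinding.
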(event Custom|TryEndTurn
  ;[0 0 0] Turn mechanics
  ;;[0.07812 0.07812 0.07812] Client
  ;;;[1 1 1] EndTurn
  (if (Variables|Default|GetItsMyTurn)
    (switch Utilities|FlowControl|Switch|SwitchonEControlMode (Variables|Default|GetControlMode)
      (:DEFAULTCONTROLS
        (Variables|Default|SetControlMode "DEFAULTCONTROLS")
        (CallFunction|SERVERRequestEndTurn))
      (:NOGAMEPLAY
        (Development|PrintString "not default controls" :!label _label))
      (:PLAYCOUNTERSPELLSONLY
        (goto _label))
      (:SELECTGROUNDLOCATION
        (goto _label))
      (:SELECTHERO
        (goto _label))
      (:SELECTMINION
        (goto _label))
      (:SELECTCHARACTER
        (goto _label)))
    (else
      (Development|PrintString "not my turn"))))

(event Custom|SERVER_PlayCard
  (params (CardToPlay :type DC%20Card%20Base%20BP%20Object%20Reference))
  ;[0 0 0] Turn mechanics
  ;;[0.07812 0.07812 0.07812] Server
  ;;;[1 1 1] Action phase : Play card
  (bind _asdcgame_mode_bp (Utilities|Casting|CastToDCGameMode_BP (Game|GetGameMode self)))
  (if (Variables|Default|GetItsMyTurn)
    (Default|PlayCard _asdcgame_mode_bp CardToPlay self)))

(event Custom|CLIENT_BeginPassiveTurn
  ;[0 0 0] Turn mechanics
  ;;[0.07812 0.07812 0.07812] Client
  ;;;[1 1 1] Turn start
  (Default|HUDUpdateHandCards (Variables|Default|GetMainUMGWidget))
  (Variables|Default|SetItsMyTurn false)
  (CallFunction|SERVERConfirmPassiveTurnStart))

(event Custom|CLIENT_BeginActiveTurn
  ;[0 0 0] Turn mechanics
  ;;[0.07812 0.07812 0.07812] Client
  ;;;[1 1 1] Turn start
  (Default|HUDUpdateHandCards (Variables|Default|GetMainUMGWidget))
  (Variables|Default|SetItsMyTurn true)
  (CallFunction|SERVERConfirmActiveTurnStart))

(event Custom|CLIENT_FinalizeEndTurn
  ;[0 0 0] Turn mechanics
  ;;[0.07812 0.07812 0.07812] Client
  ;;;[1 1 1] EndTurn
  (CallFunction|BeginNewPhase "NewEnumerator6"))

(event Custom|SERVER_ConfirmActiveTurnStart
  ;[0 0 0] Turn mechanics
  ;;[0.07812 0.07812 0.07812] Server
  ;;;[1 1 1] Turn start
  (Development|PrintString "Server : Active Turn Start confirmed" true true "(R=0.000000,G=0.171875,B=0.260417,A=1.000000)" 2e+01)
  (bind _asdcgame_mode_bp (Utilities|Casting|CastToDCGameMode_BP (Game|GetGameMode)))
  (Default|PlayerConfirmTurnStart _asdcgame_mode_bp true))

(event Custom|CLIENT_NotifyCantPlayThisCard
  ;[0 0 0] Turn mechanics
  ;;[0.07812 0.07812 0.07812] Client
  ;;;[1 1 1] Action phase
  (Development|PrintString "Can't play this card"))

(event Custom|SERVER_AnswerUpkeepRequest
  (params (UpkeepAnswer :type Boolean))
  ;[0 0 0] Turn mechanics
  ;;[0.07812 0.07812 0.07812] Server
  ;;;[1 1 1] Upkeep phase
)

(event Custom|CLIENT_RequestUpkeepDecision
  (params (UpkeepCard :type DC%20Card%20Object%20Reference))
  ;[0 0 0] Turn mechanics
  ;;[0.07812 0.07812 0.07812] Client
  ;;;[1 1 1] Upkeep phase
  (CallFunction|SERVERAnswerUpkeepRequest false))

(event Custom|SERVER_CharacterMoveToLocation
  (params (Character :type DC%20Character%20Object%20Reference) (WorldTile :type Terrain%20Tile%20Object%20Reference))
  ;[0 0 0] Turn mechanics
  ;;[0.07812 0.07812 0.07812] Server
  ;;;[1 1 1] Action phase : Play card
  (if (Variables|Default|GetItsMyTurn)
    _))

(event Custom|CLIENT_ConfirmPlaycard
  ;[0 0 0] Turn mechanics
  ;;[0.07812 0.07812 0.07812] Client
  ;;;[1 1 1] Action phase
)

(event Custom|SERVER_ConfirmPassiveTurnStart
  ;[0 0 0] Turn mechanics
  ;;[0.07812 0.07812 0.07812] Server
  ;;;[1 1 1] Turn start
  (Development|PrintString "Server : Passive Turn Start confirmed" true true "(R=0.000000,G=0.171875,B=0.260417,A=1.000000)" 2e+01)
  (bind _asdcgame_mode_bp (Utilities|Casting|CastToDCGameMode_BP (Game|GetGameMode)))
  (Default|PlayerConfirmTurnStart _asdcgame_mode_bp false))

(event Custom|CLIENT_AddCardToHand
  (params (DCCard :type DC%20Card%20Base%20BP%20Object%20Reference))
  ;[0 0 0] Turn mechanics
  ;;[0.07812 0.07812 0.07812] Server
  ;;;[1 1 1] Draw Card Phase
  (Default|HUDAddCardtoHand (Variables|Default|GetMainUMGWidget) DCCard))

(event Custom|PlayCard
  (params (CardToPlay :type DC%20Card%20Base%20BP%20Object%20Reference))
  ;[0 0 0] Turn mechanics
  ;;[0.07812 0.07812 0.07812] Client
  ;;;[1 1 1] Action phase
  (if (Variables|Default|GetItsMyTurn)
    (Variables|Default|SetControlMode "NOGAMEPLAY")
    (CallFunction|SERVERPlayCard CardToPlay)))

(event Custom|CLIENT_DisplayNewPlayedCard
  (params (DCCard :type DC%20Card%20Base%20BP%20Object%20Reference))
  ;[0 0 0] Turn mechanics
  ;;[0.07812 0.07812 0.07812] Client
  ;;;[1 1 1] Action phase
  (Default|HUDUpdatePlayedCard (Variables|Default|GetMainUMGWidget) DCCard))

(event Custom|CLIENT_RemoveCardFromHand
  (params (DCCard :type DC%20Card%20Base%20BP%20Object%20Reference))
  ;[0 0 0] Turn mechanics
  ;;[0.07812 0.07812 0.07812] Client
  ;;;[1 1 1] Action phase
  (Default|HUDRemoveCardfromHand (Variables|Default|GetMainUMGWidget) DCCard))

(event Custom|CLIENT_CounterspellRequest
  ;[0 0 0] Turn mechanics
  ;;[0.07812 0.07812 0.07812] Client
  ;;;[1 1 1] Action phase
)

(event Custom|SERVER_TryPlayCounterSpellCard
  ;[0 0 0] Turn mechanics
  ;;[0.07812 0.07812 0.07812] Server
  ;;;[1 1 1] Action phase : Play card
)

(event Custom|CLIENT_AskForSummonLocation
  ;[0 0 0] Turn mechanics
  ;;[0.07812 0.07812 0.07812] Client
  ;;;[1 1 1] Action phase
  (Variables|Default|SetControlMode "SELECTGROUNDLOCATION")
  (Development|PrintString "Select Ground Location"))

(event Custom|CLIENT_ConfirmSummon
  ;[0 0 0] Turn mechanics
  ;;[0.07812 0.07812 0.07812] Client
  ;;;[1 1 1] Action phase
  (Variables|Default|SetControlMode "DEFAULTCONTROLS"))

(event Custom|SERVER_RequestEndTurn
  ;[0 0 0] Turn mechanics
  ;;[0.07812 0.07812 0.07812] Server
  ;;;[1 1 1] EndTurn
  (bind _asdcgame_mode_bp (Utilities|Casting|CastToDCGameMode_BP (Game|GetGameMode)))
  (Default|TrytoEndTurn _asdcgame_mode_bp))

(event Custom|SERVER_TrySummonAtTerrainTile
  (params (TerrainTile :type Terrain%20Tile%20Object%20Reference))
  ;[0 0 0] Turn mechanics
  ;;[0.07812 0.07812 0.07812] Server
  ;;;[1 1 1] Action phase : Play card
  (Game|SpawnActorfromClass "/Game/Blueprint/Game/Character/PoringBP.PoringBP_C" (Math|Conversions|ToTransform(Vector) (+ (Transformation|GetActorLocation TerrainTile) "0, 0,100.000000")) "Undefined" 0 0)
  (bind _asdcgame_mode_bp (Utilities|Casting|CastToDCGameMode_BP (Game|GetGameMode)))
  (CallFunction|CLIENTConfirmSummon (Variables|/Game/Blueprint/Game/System/DCGameMode_BP.DCGameMode_BP_C|GetActivePlayerController _asdcgame_mode_bp)))

(event EventBeginPlay
  ;[0 0 0] Client
  ;;[1 1 1] BeginPlay
  (if (Pawn|IsLocalPlayerController)
    (CallFunction|CreateCamera)
    (CallFunction|SetupHud)))

(event EventTick
  (params (DeltaSeconds :type Float%20%28single-precision%29))
  (bind _array (Utilities|Array|MakeArray "ObjectTypeQuery7"))
  (bind (_hitresult _returnvalue) (Class|PlayerController|GetHitResultUnderCursorforObjects _array true))
  ;[1 1 1] Tick
  (if _returnvalue
    (bind _asterrain_tile (Utilities|Casting|CastToTerrainTile (.hitactor _hitresult)))
    (if (not (== _asterrain_tile (Variables|Default|GetHoveredOverGridTile)))
      (Utilities|IsValid (Variables|Default|GetHoveredOverGridTile)
        (:Is%20Valid
          (Rendering|SetRenderCustomDepth (Variables|/Game/Blueprint/Game/World/TerrainTile.TerrainTile_C|GetBaseCollision (Variables|Default|GetHoveredOverGridTile)) false))
        (:Is%20Not%20Valid
          _))
      (bind _output_get (Variables|Default|SetHoveredOverGridTile _asterrain_tile))
      (Rendering|SetRenderCustomDepth (Variables|/Game/Blueprint/Game/World/TerrainTile.TerrainTile_C|GetBaseCollision _output_get) true))))

(event Input|AxisEvents|InputAxisMoveForward
  (params (AxisValue :type Float%20%28single-precision%29))
  (bind _mycameraactor (Variables|Default|GetMyCameraActor))
  ;[0 0 0] Client
  ;;[1 1 1] Camera controls
  (Utilities|IsValid _mycameraactor
    (:Is%20Valid
      (Transformation|AddRelativeLocation (Variables|/Script/Engine.Actor|GetRootComponent _mycameraactor) (* (Math|Vector|GetForwardVector (Math|Rotator|MakeRotator 0.0 0.0 (.yaw (Camera|GetCameraRotation (Game|GetPlayerCameraManager 0))))) (* AxisValue 1e+01)) false false))))

(event Input|AxisEvents|InputAxisMoveRight
  (params (AxisValue :type Float%20%28single-precision%29))
  (bind _mycameraactor (Variables|Default|GetMyCameraActor))
  ;[0 0 0] Client
  ;;[1 1 1] Camera controls
  (Utilities|IsValid _mycameraactor
    (:Is%20Valid
      (Transformation|AddRelativeLocation (Variables|/Script/Engine.Actor|GetRootComponent _mycameraactor) (* (Math|Vector|GetRightVector (Math|Rotator|MakeRotator 0.0 0.0 (.yaw (Camera|GetCameraRotation (Game|GetPlayerCameraManager 0))))) (* AxisValue 1e+01)) false false))))

(event Input|MouseEvents|MouseX
  (params (AxisValue :type Float%20%28single-precision%29))
  (bind (_sizex _sizey) (HUD|GetViewportSize))
  (bind _mycameraactor (Variables|Default|GetMyCameraActor))
  (bind _springarm (Variables|/Game/Blueprint/Game/DCCameraPawn.DCCameraPawn_C|GetSpringArm _mycameraactor))
  (bind _relativerotation (Variables|/Script/Engine.SceneComponent|GetRelativeRotation _springarm))
  ;[0 0 0] Client
  ;;[1 1 1] Camera controls
  (if (Variables|Default|GetRightMouseButtonClicked)
    (Class|PlayerController|SetMouseLocation (/ _sizex 2) (/ _sizey 2))
    (Transformation|SetRelativeRotation _springarm (Math|Rotator|MakeRotator 0.0 (Math|Float|Clamp(Float) (+ (.pitch _relativerotation) (* (stale Input|MouseEvents|MouseY AxisValue) 1.0)) -8e+01 -2e+01) (+ (.yaw _relativerotation) (* AxisValue 2.0))) false false)))

(event Input|MouseEvents|MouseWheelAxis
  (params (AxisValue :type Float%20%28single-precision%29))
  (bind _mycameraactor (Variables|Default|GetMyCameraActor))
  (bind _springarm (Variables|/Game/Blueprint/Game/DCCameraPawn.DCCameraPawn_C|GetSpringArm _mycameraactor))
  ;[0 0 0] Client
  ;;[1 1 1] Camera controls
  (Variables|/Script/Engine.SpringArmComponent|SetTargetArmLength _springarm (Math|Float|Clamp(Float) (+ (* AxisValue -1e+02) (Variables|/Script/Engine.SpringArmComponent|GetTargetArmLength _springarm)) 2e+02 3e+03)))

(event Input|MouseEvents|MouseY
  (params (AxisValue :type Float%20%28single-precision%29))
  (bind (_sizex _sizey) (HUD|GetViewportSize))
  (bind _mycameraactor (Variables|Default|GetMyCameraActor))
  (bind _springarm (Variables|/Game/Blueprint/Game/DCCameraPawn.DCCameraPawn_C|GetSpringArm _mycameraactor))
  (bind _relativerotation (Variables|/Script/Engine.SceneComponent|GetRelativeRotation _springarm))
  ;[0 0 0] Client
  ;;[1 1 1] Camera controls
  (if (Variables|Default|GetRightMouseButtonClicked)
    (Class|PlayerController|SetMouseLocation (/ _sizex 2) (/ _sizey 2))
    (Transformation|SetRelativeRotation _springarm (Math|Rotator|MakeRotator 0.0 (Math|Float|Clamp(Float) (+ (.pitch _relativerotation) (* AxisValue 1.0)) -8e+01 -2e+01) (+ (.yaw _relativerotation) (* (stale Input|MouseEvents|MouseX AxisValue) 2.0))) false false)))

(event Input|KeyboardEvents|Q
  (params (Key :type Key%20Structure))
  ;[0 0 0] Client
  ;;[1 1 1] Quit game
  (:Pressed
    (Game|QuitGame self "Quit")))

(event Input|KeyboardEvents|P
  (params (Key :type Key%20Structure))
  ;[0 0 0] Client
  (:Pressed
    (bind _returnvalue (Class|NavigationSystem|FindPathtoLocationSynchronously (Math|Vector|MakeVector 0.0 0.0 0.0) (.location (.HitResult (Game|Player|GetHitResultUnderCursorbyChannel "TraceTypeQuery1" true))) self))
    (for _array_element (Variables|/Script/Engine.NavigationPath|GetPathPoints _returnvalue)
      (Rendering|Debug|DrawDebugSphere _array_element 1e+01 12 "(R=1.000000,G=1.000000,B=1.000000,A=1.000000)" 2.0 1.0))))

(event Input|KeyboardEvents|R
  (params (Key :type Key%20Structure))
  (bind _returnvalue (Math|Vector|MakeVector -1.8e+03 1.7e+03 0.0))
  (bind _array (Utilities|Array|MakeArray "ObjectTypeQuery1"))
  (bind (_hitresult _returnvalue_2) (Class|PlayerController|GetHitResultUnderCursorforObjects _array true))
  (:Pressed
    (if _returnvalue_2
      (Rendering|Debug|DrawDebugSphere (.location _hitresult) 1e+02 12 "(R=1.000000,G=1.000000,B=1.000000,A=1.000000)" 0.0)
      (bind (_pathpoints _returnvalue_3) (Class|NavLocalGridManager|FindLocalNavigationGridPath _returnvalue (.location _hitresult)))
      (if _returnvalue_3
        (for _array_element _pathpoints
          (Rendering|Debug|DrawDebugLine _returnvalue _array_element "(R=0.000000,G=0.000000,B=0.000000,A=1.000000)" 1e+01 5.0))
        (else
          (Development|PrintString "no path"))))))

(event Input|KeyboardEvents|J
  (params (Key :type Key%20Structure))
  (:Pressed
    (bind _asterrain_tile (Utilities|Casting|CastToTerrainTile (Variables|Default|GetHoveredOverGridTile)))
    (Utilities|IsValid _asterrain_tile
      (:Is%20Valid
        (bind _outactors (Actor|GetAllActorsOfClass "/Game/Blueprint/Game/Character/GridPathAiController_BP.GridPathAiController_BP_C"))
        (for _array_element _outactors
          (Default|NewFunction0 _array_element (Transformation|GetActorLocation _asterrain_tile)))))))

(event Input|MouseEvents|LeftMouseButton
  (params (Key :type Key%20Structure))
  ;[0 0 0] Client
  ;;[1 1 1] Left Mouse Button
  (:Pressed
    (CallFunction|LeftClick)))

(event Input|MouseEvents|RightMouseButton
  (params (Key :type Key%20Structure))
  (bind (_locationx _locationy) (Game|Player|GetMousePosition))
  ;[0 0 0] Client
  ;;[1 1 1] Camera controls
  (:Pressed
    (Variables|Default|SetSavedMousePos (Math|Vector2D|MakeVector2D _locationx _locationy))
    (Variables|Default|SetRightMouseButtonClicked true)
    (Variables|Default|SetbShowMouseCursor false))
  (:Released
    (Class|PlayerController|SetMouseLocation (Math|Float|Truncate (.x (Variables|Default|GetSavedMousePos))) (Math|Float|Truncate (.y (Variables|Default|GetSavedMousePos))))
    (Variables|Default|SetRightMouseButtonClicked false)
    (Variables|Default|SetbShowMouseCursor true)))

(fn ConstructionScript)

(fn CreateCamera
  (bind _returnvalue (Game|SpawnActorfromClass "/Game/Blueprint/Game/DCCameraPawn.DCCameraPawn_C" (Math|Transform|MakeTransform "0, 0,50.000000") "AlwaysSpawn" self 0))
  (Game|Player|SetViewTargetwithBlend _returnvalue 0.0 "VTBlend_Linear" 0.0 false)
  (Variables|Default|SetMyCameraActor _returnvalue)
  (Development|PrintString "camera created")
  (return))

(fn SetupHud
  (bind _returnvalue (UserInterface|CreateWidget "/Game/Blueprint/Game/Ui/W_TestHud_BP.W_TestHud_BP_C" self))
  (UserInterface|Viewport|AddtoViewport _returnvalue 0)
  (Variables|Default|SetMainUMGWidget _returnvalue))

(fn BeginActiveTurn
  (Variables|Default|SetItsMyTurn true)
  (Variables|Default|SetControlMode "DEFAULTCONTROLS")
  (Development|PrintString "it's my turn! :)" true true "(R=0.000000,G=0.660000,B=1.000000,A=1.000000)" 2e+01)
  (CallFunction|SERVERConfirmActiveTurnStart))

(fn BeginPassiveTurn
  (Variables|Default|SetItsMyTurn false)
  (Variables|Default|SetControlMode "DEFAULTCONTROLS")
  (Development|PrintString "not my turn..." true true "(R=0.000000,G=0.660000,B=1.000000,A=1.000000)" 2e+01))

(fn BeginNewPhase
  (params (NewPhase :type ETurnPhase%20Enum :default "NewEnumerator1"))
  (Development|PrintString (Utilities|String|Append "Client : New phase : " (Utilities|String|EnumtoString NewPhase)) true true "(R=0.510417,G=0.032757,B=0.000000,A=1.000000)" 3e+01)
  (Default|HUDUpdatewithPhaseChange (Variables|Default|GetMainUMGWidget) NewPhase (Variables|Default|GetItsMyTurn))
  (switch Utilities|FlowControl|Switch|SwitchonETurnPhase NewPhase
    (:NewEnumerator1
      (CallFunction|PhaseUpkeepBegin))
    (:NewEnumerator2
      (CallFunction|PhasePermaEffectsBegin))
    (:NewEnumerator3
      (CallFunction|PhaseDrawCardBegin))
    (:NewEnumerator4
      (CallFunction|PhaseActionBegin))
    (:NewEnumerator6
      (CallFunction|BeginEndTurn))))

(fn BeginEndTurn
  (Variables|Default|SetItsMyTurn false)
  (Development|PrintString "Finalize End Turn" true true "(R=0.510417,G=0.032757,B=0.000000,A=1.000000)" 3e+01)
  (Variables|Default|SetControlMode "DEFAULTCONTROLS")
  (Default|HUDClearPlayedCard (Variables|Default|GetMainUMGWidget)))

(fn PhaseUpkeepBegin
  (Variables|Default|SetControlMode "DEFAULTCONTROLS"))

(fn PhaseUpkeepContinue)

(fn PhasePermaEffectsBegin
  (Variables|Default|SetControlMode "DEFAULTCONTROLS"))

(fn PhasePermaEffectsContinue)

(fn PhaseDrawCardBegin
  (Variables|Default|SetControlMode "NOGAMEPLAY")
  (Default|HUDUpdateHandCards (Variables|Default|GetMainUMGWidget)))

(fn PhaseDrawCardContinue)

(fn PhaseActionBegin
  (Variables|Default|SetControlMode "DEFAULTCONTROLS"))

(fn PhaseActionContinue)

(fn LeftClick
  (switch Utilities|FlowControl|Switch|SwitchonEControlMode (Variables|Default|GetControlMode)
    (:SELECTGROUNDLOCATION
      (bind _asterrain_tile (Utilities|Casting|CastToTerrainTile (.hitactor (.HitResult (Class|PlayerController|GetHitResultUnderCursorforObjects (Utilities|Array|MakeArray "ObjectTypeQuery7" "ObjectTypeQuery8") true)))))
      (if (Variables|/Game/Blueprint/Game/World/TerrainTile.TerrainTile_C|GetbTraversible _asterrain_tile)
        (CallFunction|SERVERTrySummonatTerrainTile _asterrain_tile)
        (else
          (Development|PrintString "No"))))))