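; DCPlayerState_BP is a player state Blueprint that tracks a player's card collections in a card game, namely a Hand and a Graveyard.
; Small functions add a card to the hand, remove one from it, or add one to the graveyard.
; MoveCardFromHandToGraveyard chains the remove and graveyard-add calls to discard a card.
; It has no active event logic.
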(event EventBeginPlay)

(event EventTick
  (params (DeltaSeconds :type Float%20%28single-precision%29)))

(fn ConstructionScript)

(fn RemoveCardfromHand
  (params (CardToRemove :type DC%20Card%20Base%20BP%20Object%20Reference))
  (Utilities|Array|RemoveItem (Variables|Default|GetHand) CardToRemove)
  (return))

(fn AddCardtoHand
  (params (CardToAdd :type DC%20Card%20Base%20BP%20Object%20Reference))
  (Utilities|Array|Add (Variables|Default|GetHand) CardToAdd)
  (return))

(fn AddCardtoGraveYard
  (params (CardToAdd :type DC%20Card%20Base%20BP%20Object%20Reference))
  (Utilities|Array|Add (Variables|Default|GetGraveyard) CardToAdd)
  (return))

(fn MoveCardfromHandtoGraveyard
  (params (Card :type DC%20Card%20Base%20BP%20Object%20Reference))
  (CallFunction|RemoveCardfromHand Card)
  (CallFunction|AddCardtoGraveYard Card)
  (return))