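; Game state Blueprint for a turn-based card game that tracks the current turn phase and the stack of played cards.
; BeginPlay caches player controller 0, and MULTICAST_BeginNewPhase stores the new phase and forwards it to that index's DCPlayerController_BP.
; AddCardToPlayedCardStack appends a card to CurrentlyPlayedCards and prints a debug count from the add result.
; The resume-phase and end-turn multicast events are empty stubs.
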(event Custom|MULTICAST_BeginNewPhase
  (params (NewTurnPhase :type ETurnPhase%20Enum :default "NewEnumerator1"))
  (bind _output_get (Variables|Default|SetCurrentPhase NewTurnPhase))
  (bind _asdcplayer_controller_bp (Utilities|Casting|CastToDCPlayerController_BP (Game|GetPlayerController 0)))
  (Default|BeginNewPhase _asdcplayer_controller_bp _output_get))

(event Custom|MULTICAST_ResumePhase
  (params (ResumeTurnPhase :type ETurnPhase%20Enum :default "NewEnumerator1")))

(event Custom|MULTICAST_EndTurn)

(event EventBeginPlay
  (bind _asdcplayer_controller_bp (Utilities|Casting|CastToDCPlayerController_BP (Game|GetPlayerController 0)))
  (Variables|Default|SetMyPlayerController _asdcplayer_controller_bp)
  (Development|PrintString "gamestate set new player controller"))

(event EventTick
  (params (DeltaSeconds :type Float%20%28single-precision%29)))

(fn ConstructionScript)

(fn AddCardtoPlayedCardStack
  (params (PlayedCard :type DC%20Card%20Base%20BP%20Object%20Reference))
  (bind _returnvalue (Utilities|Array|Add (Variables|Default|GetCurrentlyPlayedCards) PlayedCard))
  (Development|PrintString (Utilities|String|Append "Now this many cards on played card stack : " (Utilities|String|ToString(Integer) _returnvalue)))
  (return))