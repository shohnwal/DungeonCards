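; WorldGrid_BP is a world grid actor that spawns and manages TerrainTile actors laid out by X/Y coordinate.
; Events rebuild the grid, grow or shrink it by a row or column, and refresh meshes.
; Refreshing redraws trees as randomly rotated and scaled HISM instances and sets those tiles non-traversible.
; The terrain cube pass exists but is never called here, and SetupTraversibility is empty.
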(event Custom|Grid%20ReBuild
  (CallFunction|RebuildWorld))

(event Custom|Remove
  (Actor|DestroyActor)
  (Components|InstancedStaticMesh|ClearInstances (Variables|Default|GetTree1_HISMC)))

(event Custom|MeshesRefresh
  (CallFunction|DevRefreshMeshes))

(event Custom|Grid:Y++
  (bind _worldsize (Variables|Default|GetWorldSize))
  (for _index (range 1 (.x _worldsize))
    (CallFunction|DevBuildTile _index (+ (.y _worldsize) 1)))
  (Math|Integer|IncrementInt (.y _worldsize)))

(event Custom|Grid:Y--
  (bind (_arrayindex _arrayelement) (Utilities|Array|ReverseforEachLoop (Variables|Default|GetWorldTiles))
    (:LoopBody
      (if (== (.y (Variables|/Game/Blueprint/Game/World/TerrainTile.TerrainTile_C|GetGridCoordinate _arrayelement)) (.y (Variables|Default|GetWorldSize)))
        (Actor|DestroyActor _arrayelement)
        (Utilities|Array|RemoveIndex (Variables|Default|GetWorldTiles) _arrayindex)))
    (:Completed
      (Math|Integer|DecrementInt (.y (Variables|Default|GetWorldSize))
        (:%20%20
          (CallFunction|DevRefreshMeshes))))))

(event Custom|Grid:X++
  (bind _worldsize (Variables|Default|GetWorldSize))
  (for _index (range 1 (.y _worldsize))
    (CallFunction|DevBuildTile (+ (.x _worldsize) 1) _index))
  (Math|Integer|IncrementInt (.x _worldsize)))

(event Custom|Grid:X--
  (bind (_arrayindex _arrayelement) (Utilities|Array|ReverseforEachLoop (Variables|Default|GetWorldTiles))
    (:LoopBody
      (if (== (.x (Variables|/Game/Blueprint/Game/World/TerrainTile.TerrainTile_C|GetGridCoordinate _arrayelement)) (.x (Variables|Default|GetWorldSize)))
        (Actor|DestroyActor _arrayelement)
        (Utilities|Array|RemoveIndex (Variables|Default|GetWorldTiles) _arrayindex)))
    (:Completed
      (Math|Integer|DecrementInt (.x (Variables|Default|GetWorldSize))
        (:%20%20
          (CallFunction|DevRefreshMeshes))))))

(event EventBeginPlay)

(event Collision|EventActorBeginOverlap
  (params (OtherActor :type Actor%20Object%20Reference)))

(event EventDestroyed
  (for _array_element (Variables|Default|GetWorldTiles)
    (Actor|DestroyActor _array_element)))

(event EventTick
  (params (DeltaSeconds :type Float%20%28single-precision%29)))

(fn ConstructionScript)

(fn CreateGrid
  (bind _worldsize (Variables|Default|GetWorldSize))
  (for _index (range 1 (.x _worldsize))
    (for _index_2 (range 1 (.y _worldsize))
      (CallFunction|DevBuildTile _index _index_2))))

(fn RebuildWorld
  (bind _worldtiles (Variables|Default|GetWorldTiles))
  (Components|InstancedStaticMesh|ClearInstances (Variables|Default|GetTree1_HISMC))
  (for _array_element _worldtiles
    (Actor|DestroyActor _array_element))
  (Utilities|Array|Clear _worldtiles)
  (CallFunction|CreateGrid))

(fn DevRefreshMeshes
  (Components|InstancedStaticMesh|ClearInstances (Variables|Default|GetTree1_HISMC))
  (Components|InstancedStaticMesh|ClearInstances (Variables|Default|GetTerrainCube_HISMC))
  (for _array_element (Variables|Default|GetWorldTiles)
    (CallFunction|GenerateTerrainChildMesh _array_element)))

(fn DevBuildTile
  (params (X :type Integer) (Y :type Integer))
  (bind _returnvalue (Transformation|GetActorLocation))
  (bind _returnvalue_2 (Game|SpawnActorfromClass "/Game/Blueprint/Game/World/TerrainTile.TerrainTile_C" (Math|Transform|MakeTransform (Math|Vector|MakeVector (+ (.x _returnvalue) (Math|Conversions|ToFloat(Integer) (* X 300))) (+ (.y _returnvalue) (Math|Conversions|ToFloat(Integer) (* Y 300))) 0.0)) "Undefined" 0 0))
  (Variables|/Game/Blueprint/Game/World/TerrainTile.TerrainTile_C|SetGridCoordinate _returnvalue_2 (Utilities|Struct|MakeIntVector X Y 0))
  (Utilities|Array|Add (Variables|Default|GetWorldTiles) _returnvalue_2)
  (Transformation|AttachActorToActor _returnvalue_2 self "None" "KeepRelative" "KeepRelative" "KeepRelative" false))

(fn GenerateTerrainBaseMesh
  (params (WorldTile :type Terrain%20Tile%20Object%20Reference))
  (switch Utilities|FlowControl|Switch|SwitchonETerrainTileBaseMesh (Variables|/Game/Blueprint/Game/World/TerrainTile.TerrainTile_C|GetTerrainBaseMeshType WorldTile)
    (:NewEnumerator0
      (Class|InstancedStaticMeshComponent|AddInstanceWorldSpace (Variables|Default|GetTerrainCube_HISMC) (Math|Transform|MakeTransform (+ (Transformation|GetActorLocation WorldTile) "0, 0,-150.000000") (Math|Rotator|MakeRotator 0.0 0.0 0.0) (Math|Vector|MakeVector 3.0 3.0 3.0)))
      (Development|PrintString "Hello"))))

(fn GenerateTerrainChildMesh
  (params (WorldTile :type Terrain%20Tile%20Object%20Reference))
  (bind _returnvalue (Math|Random|RandomFloatinRange 0.7 1.2))
  (switch Utilities|FlowControl|Switch|SwitchonETerrainTileChildMesh (Variables|/Game/Blueprint/Game/World/TerrainTile.TerrainTile_C|GetTerrainChildMeshType WorldTile)
    (:NewEnumerator1
      (Variables|/Game/Blueprint/Game/World/TerrainTile.TerrainTile_C|SetbTraversible WorldTile true))
    (:NewEnumerator0
      (Variables|/Game/Blueprint/Game/World/TerrainTile.TerrainTile_C|SetbTraversible WorldTile false)
      (Class|InstancedStaticMeshComponent|AddInstanceWorldSpace (Variables|Default|GetTree1_HISMC) (Math|Transform|MakeTransform (Transformation|GetActorLocation WorldTile) (Math|Rotator|MakeRotator 0.0 0.0 (.yaw (Math|Random|RandomRotator false))) (Math|Vector|MakeVector _returnvalue _returnvalue _returnvalue)))
      (Development|PrintString "Hello"))))

(fn SetupTraversibility)