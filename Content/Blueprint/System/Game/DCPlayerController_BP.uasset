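; Player controller that spawns a free camera pawn and test HUD for the local player, then drives the camera.
; Movement axes pan it relative to view yaw, the wheel zooms the spring arm, and right-drag rotates it with the cursor hidden and later restored.
; Tick traces hovered pawns for click printing.
; Debug keys draw navigation paths, add cards to player state and quit; SERVER_TryUseCard is a stub.
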(event Custom|SERVER_TryUseCard
  (Utilities|Casting|CastToDCGameMode_BP (Game|GetGameMode)))

(event EventBeginPlay
  (bind _self self)
  (if (Pawn|IsLocalPlayerController _self)
    (bind _returnvalue (Game|SpawnActorfromClass "/Game/Blueprint/DCCameraPawn.DCCameraPawn_C" (Math|Transform|MakeTransform "0, 0,50.000000") "Undefined" _self 0))
    (Game|Player|SetViewTargetwithBlend _returnvalue 0.0 "VTBlend_Linear" 0.0 false)
    (Variables|Default|SetMyCameraActor _returnvalue)
    (bind _returnvalue_2 (UserInterface|CreateWidget "/Game/Blueprint/Ui/Game/W_TestHud_BP.W_TestHud_BP_C"))
    (UserInterface|Viewport|AddtoViewport _returnvalue_2 0)))

(event EventTick
  (params (DeltaSeconds :type Float%20%28single-precision%29))
  (bind _array (Utilities|Array|MakeArray "ObjectTypeQuery3"))
  (bind (_hitresult _returnvalue) (Class|PlayerController|GetHitResultUnderCursorforObjects _array true))
  (if _returnvalue
    (Variables|Default|SetHoveredOverActor (.hitactor _hitresult))
    (else
      (Variables|Default|SetHoveredOverActor 0))))

(event Input|AxisEvents|InputAxisMoveForward
  (params (AxisValue :type Float%20%28single-precision%29))
  (bind _mycameraactor (Variables|Default|GetMyCameraActor))
  ;[1 1 1] Movement
  (Utilities|IsValid _mycameraactor
    (:Is%20Valid
      (Transformation|AddRelativeLocation (Variables|/Script/Engine.Actor|GetRootComponent _mycameraactor) (* (Math|Vector|GetForwardVector (Math|Rotator|MakeRotator 0.0 0.0 (.yaw (Camera|GetCameraRotation (Game|GetPlayerCameraManager 0))))) (* AxisValue 1e+01)) false false))))

(event Input|AxisEvents|InputAxisMoveRight
  (params (AxisValue :type Float%20%28single-precision%29))
  (bind _mycameraactor (Variables|Default|GetMyCameraActor))
  ;[1 1 1] Movement
  (Utilities|IsValid _mycameraactor
    (:Is%20Valid
      (Transformation|AddRelativeLocation (Variables|/Script/Engine.Actor|GetRootComponent _mycameraactor) (* (Math|Vector|GetRightVector (Math|Rotator|MakeRotator 0.0 0.0 (.yaw (Camera|GetCameraRotation (Game|GetPlayerCameraManager 0))))) (* AxisValue 1e+01)) false false))))

(event Input|MouseEvents|MouseX
  (params (AxisValue :type Float%20%28single-precision%29))
  (bind (_sizex _sizey) (HUD|GetViewportSize))
  (bind _mycameraactor (Variables|Default|GetMyCameraActor))
  (bind _springarm (Variables|/Game/Blueprint/DCCameraPawn.DCCameraPawn_C|GetSpringArm _mycameraactor))
  (bind _relativerotation (Variables|/Script/Engine.SceneComponent|GetRelativeRotation _springarm))
  (if (Variables|Default|GetRightMouseButtonClicked)
    (Class|PlayerController|SetMouseLocation (/ _sizex 2) (/ _sizey 2))
    (Transformation|SetRelativeRotation _springarm (Math|Rotator|MakeRotator 0.0 (Math|Float|Clamp(Float) (+ (.pitch _relativerotation) (* (stale Input|MouseEvents|MouseY AxisValue) 1.0)) -8e+01 -2e+01) (+ (.yaw _relativerotation) (* AxisValue 2.0))) false false)))

(event Input|MouseEvents|MouseWheelAxis
  (params (AxisValue :type Float%20%28single-precision%29))
  (bind _mycameraactor (Variables|Default|GetMyCameraActor))
  (bind _springarm (Variables|/Game/Blueprint/DCCameraPawn.DCCameraPawn_C|GetSpringArm _mycameraactor))
  (Variables|/Script/Engine.SpringArmComponent|SetTargetArmLength _springarm (Math|Float|Clamp(Float) (+ (* AxisValue -1e+02) (Variables|/Script/Engine.SpringArmComponent|GetTargetArmLength _springarm)) 2e+02 3e+03)))

(event Input|MouseEvents|MouseY
  (params (AxisValue :type Float%20%28single-precision%29))
  (bind (_sizex _sizey) (HUD|GetViewportSize))
  (bind _mycameraactor (Variables|Default|GetMyCameraActor))
  (bind _springarm (Variables|/Game/Blueprint/DCCameraPawn.DCCameraPawn_C|GetSpringArm _mycameraactor))
  (bind _relativerotation (Variables|/Script/Engine.SceneComponent|GetRelativeRotation _springarm))
  (if (Variables|Default|GetRightMouseButtonClicked)
    (Class|PlayerController|SetMouseLocation (/ _sizex 2) (/ _sizey 2))
    (Transformation|SetRelativeRotation _springarm (Math|Rotator|MakeRotator 0.0 (Math|Float|Clamp(Float) (+ (.pitch _relativerotation) (* AxisValue 1.0)) -8e+01 -2e+01) (+ (.yaw _relativerotation) (* (stale Input|MouseEvents|MouseX AxisValue) 2.0))) false false)))

(event Input|KeyboardEvents|Q
  (params (Key :type Key%20Structure))
  (:Pressed
    (Game|QuitGame self "Quit")))

(event Input|KeyboardEvents|P
  (params (Key :type Key%20Structure))
  (:Pressed
    (bind _returnvalue (Class|NavigationSystem|FindPathtoLocationSynchronously (Math|Vector|MakeVector 0.0 0.0 0.0) (.location (.HitResult (Game|Player|GetHitResultUnderCursorbyChannel "TraceTypeQuery1" true))) self))
    (for _array_element (Variables|/Script/Engine.NavigationPath|GetPathPoints _returnvalue)
      (Rendering|Debug|DrawDebugSphere _array_element 1e+01 12 "(R=1.000000,G=1.000000,B=1.000000,A=1.000000)" 2.0 1.0))))

(event Input|KeyboardEvents|C
  (params (Key :type Key%20Structure))
  (:Pressed
    (bind _asdcplayer_state_bp (Utilities|Casting|CastToDCPlayerState_BP (Variables|GetPlayerState))
      (:then
        (bind _returnvalue (Class|DCCard|SpawnCardObject))
        (Utilities|Array|Add (Variables|/Game/Blueprint/System/Game/DCPlayerState_BP.DCPlayerState_BP_C|GetMyCards _asdcplayer_state_bp) _returnvalue))
      (:CastFailed
        (Development|PrintString "cast failed")))))

(event Input|MouseEvents|LeftMouseButton
  (params (Key :type Key%20Structure))
  (bind _hoveredoveractor (Variables|Default|GetHoveredOverActor))
  (:Pressed
    (Utilities|IsValid _hoveredoveractor
      (:Is%20Valid
        (Development|PrintString (Class|KismetSystemLibrary|GetPathName _hoveredoveractor))))))

(event Input|MouseEvents|RightMouseButton
  (params (Key :type Key%20Structure))
  (bind (_locationx _locationy) (Game|Player|GetMousePosition))
  (:Pressed
    (Variables|Default|SetSavedMousePos (Math|Vector2D|MakeVector2D _locationx _locationy))
    (Variables|Default|SetRightMouseButtonClicked true)
    (Variables|Default|SetbShowMouseCursor false))
  (:Released
    (Class|PlayerController|SetMouseLocation (Math|Float|Truncate (.x (Variables|Default|GetSavedMousePos))) (Math|Float|Truncate (.y (Variables|Default|GetSavedMousePos))))
    (Variables|Default|SetRightMouseButtonClicked false)
    (Variables|Default|SetbShowMouseCursor true)))

(fn ConstructionScript)