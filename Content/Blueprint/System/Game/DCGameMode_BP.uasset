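; DCGameMode_BP is a game mode Blueprint for a multiplayer card game, still largely unfinished.
; PostLogin prints whether the new player is server or client, judged by a player controller ID of zero.
; TryUseCard checks that the card is in the player state's MyCards, then switches on card type with no actions connected.
; The confirm-use event is empty, and nodes for adding cards and confirming use are left unconnected.
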(event Custom|TryUseCard
  (params (CardToUse :type DC%20Card%20Object%20Reference) (DCPlayerController :type DC%20Player%20Controller%20BP%20Object%20Reference))
  ;[1 1 1] Check if player has the card
  (bind _asdcplayer_state_bp (Utilities|Casting|CastToDCPlayerState_BP (Variables|/Script/Engine.Controller|GetPlayerState DCPlayerController)))
  (if (Utilities|Array|ContainsItem (Variables|/Game/Blueprint/System/Game/DCPlayerState_BP.DCPlayerState_BP_C|GetMyCards _asdcplayer_state_bp) CardToUse)
    (switch Utilities|FlowControl|Switch|SwitchonECardType (Variables|/Script/DungeonCards.DCCard|GetCardType CardToUse))))

(event Custom|CLIENT_ConfirmUseCard
  (params (NewParam :type DC%20Player%20Controller%20BP%20Object%20Reference)))

(event EventBeginPlay)

(event EventTick
  (params (DeltaSeconds :type Float%20%28single-precision%29)))

(event EventPostLogin
  (params (NewPlayer :type Player%20Controller%20Object%20Reference))
  (bind _returnvalue (Class|GameplayStatics|GetPlayerControllerID NewPlayer))
  (if (== _returnvalue 0)
    (Development|PrintString "IsServer")
    (else
      (Development|PrintString "IsClient"))))

(fn ConstructionScript)